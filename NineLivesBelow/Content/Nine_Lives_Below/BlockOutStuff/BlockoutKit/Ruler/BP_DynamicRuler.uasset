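; BP_DynamicRuler is a blockout ruler actor that displays a configurable length in the level.
; Its construction script stretches LengthCube along X by LengthScale at a thin fixed cross-section and resets RulerEnd to unit world scale.
; Two text components show the length in Unreal units (LengthScale times 100) and in meters (the raw LengthScale).
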(fn `UserConstructionScript`
  (bind _lengthscale (`self.LengthScale`))
  (`SceneComponent.SetWorldScale3D` (`self.LengthCube`) (`KismetMathLibrary.MakeVector` _lengthscale 0.2 0.2))
  (`SceneComponent.SetWorldScale3D` (`self.RulerEnd`) (1.0 1.0 1.0))
  (`TextRenderComponent.K2_SetText` (`self.Distance UUs`) (`KismetTextLibrary.Conv_DoubleToText` (* _lengthscale 100.0) "HalfToEven"))
  (`TextRenderComponent.K2_SetText` (`self.Distance Meters`) (`KismetTextLibrary.Conv_DoubleToText` _lengthscale "HalfToEven")))