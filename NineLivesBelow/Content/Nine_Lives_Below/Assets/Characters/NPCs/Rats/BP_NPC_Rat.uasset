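; Rat NPC that reacts to the player (Jenny) and can be captured, extending a parent NPC's notice and passive behaviors.
; Notice events and heard noises set its state and push it, with the player reference, to the AI blackboard.
; Returning to passive waits on a retriggerable delay.
; Capture flags the blackboard, then hides the rat and disables its collision, movement and pawn sensing instead of destroying it, with no restore logic.
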(event `self.ReceiveBeginPlay`
  ;[0.8204 1 0.7841] On Begin Play, get reference to the blackboard and behavior tree!
  (`parent.ReceiveBeginPlay`)
  (set `self.Rat_BB` (`AIBlueprintHelperLibrary.GetBlackboard` (`AIBlueprintHelperLibrary.GetAIController` self))))

(event `self.Set Notice Mode`
  ;[0.2502 1 0.7991] Behaviors to play when the NPC notices the player!
  (`parent.Set Notice Mode`)
  (set `self.NPC_State` "NewEnumerator0" :!label _label)
  ;[6.2e-05 0.142 0.15 0.5] Update the Blackboard's NPC State Enum/Jenny Ref with the BP's values!
  (`BlackboardComponent.SetValueAsEnum` (`self.Rat_BB`) "NPC_State" (`self.NPC_State`) :!label _label_2)
  (bind _jennyref (`self.JennyRef`)
    (:`then`
      (`BlackboardComponent.SetValueAsObject` (`self.Rat_BB`) "JennyRef" _jennyref))
    (:`else`
      (bind _output_get (set `self.JennyRef` (`GameplayStatics.GetPlayerPawn` 0)))
      (`BlackboardComponent.SetValueAsObject` (`self.Rat_BB`) "JennyRef" _output_get))))

(event `self.NoiseHeard`
  (params (Instigator :type "Pawn Object Reference") (Location :type "Vector Structure") (Volume :type "Float (double-precision)"))
  ;[0.2502 1 0.7991] Behaviors to play when the NPC notices the player!
  ;;[0.6172 0.6514 0.8632 0.502] TO DO: If PawnSensing detects a noise, the rat goes to its EQS TargetLocation!
  (`KismetSystemLibrary.PrintString` "A rat has heard you. It has been set to Notice Mode!" true true (struct :`R` 0.617207 :`G` 0.651406 :`B` 0.863157 :`A` 0.501961))
  (`self.NoticeSequence` Instigator)
  (goto _label))

(event `self.Set Passive Mode`
  ;[0.062 0.1771 0.1374] Behaviors to play when the NPC no longer notices the player!
  (`KismetSystemLibrary.RetriggerableDelay` 3.0)
  (switch `/Game/Nine_Lives_Below/Assets/Characters/NPCs/E_NPC_State` (`self.NPC_State`)
    (:`NewEnumerator0`
      (`parent.Set Passive Mode`)
      (set `self.NPC_State` "NewEnumerator1")
      (goto _label_2))))

(event `/Game/Nine_Lives_Below/Assets/Blueprints/Interfaces/BPI_Capturable.OnCapture`
  ;[0.15 0.1248 0.06663 0.502] When captured, the rat's mesh, movement, behavior tree and pawn sensing are all turned off!
  (`KismetSystemLibrary.PrintString` "RAT CAPTURED! The rat is now turned off!" true true (struct :`R` 0.417391 :`G` 1.0 :`B` 0.078261 :`A` 1.0))
  (bind _output_get (set `self.IsCaptured` true))
  (`self.ChangeCaptureStatus` _output_get))

(fn `ChangeCaptureStatus`
  (params (IsCaptured :type Boolean))
  (bind _pawnsensing (`self.PawnSensing`))
  (`BlackboardComponent.SetValueAsBool` (`self.Rat_BB`) "IsCaptured" IsCaptured)
  ;[0.15 0.1248 0.06663 0.502] If the rat is captured, turn off its collision, pawn sensing, mini-map icon and model. If not, don't!
  (if IsCaptured
    (`PrimitiveComponent.SetCollisionResponseToAllChannels` (`self.Mesh`) "ECR_Ignore")
    (`SceneComponent.SetVisibility` (`self.CapsuleComponent`) false true)
    (`ActorComponent.Deactivate` (`self.CharacterMovement`))
    (set `PawnSensingComponent.bSeePawns` false _pawnsensing)
    (set `PawnSensingComponent.bHearNoises` false _pawnsensing)
    (`PrimitiveComponent.SetCollisionResponseToAllChannels` (`self.CapsuleComponent`) "ECR_Ignore")
    (`PrimitiveComponent.SetCollisionObjectType` (`self.CapsuleComponent`) "ECC_PhysicsBody")
    (`PrimitiveComponent.SetCollisionObjectType` (`self.Mesh`) "ECC_PhysicsBody")))

(fn `UserConstructionScript`
  (`parent.UserConstructionScript`))